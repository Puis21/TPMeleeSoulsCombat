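; Behavior tree service that picks the current behavior for a BP_MasterAI enemy and writes it to a blackboard enum key.
; On search start it caches the controller and pawn, and on activation it resets the behavior to Nothing.
; Each tick it chooses Attacking or Chasing by distance to the blackboard target, Patrolling without a target, and Nothing when the state manager reports Dead.
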(event EventReceiveTickAI
  (params (OwnerController :type AI%20Controller%20Object%20Reference) (ControlledPawn :type Pawn%20Object%20Reference) (DeltaSeconds :type Float%20%28single-precision%29))
  (CallFunction|UpdateBehavior))

(event EventReceiveSearchStartAI
  (params (OwnerController :type AI%20Controller%20Object%20Reference) (ControlledPawn :type Pawn%20Object%20Reference))
  (bind _asbp_master_ai (Utilities|Casting|CastToBP_MasterAI ControlledPawn))
  (Variables|Default|SetControlled%20MasterAI _asbp_master_ai)
  (Variables|Default|SetOwner%20Controller OwnerController))

(event EventReceiveActivation
  (params (OwnerActor :type Actor%20Object%20Reference))
  (CallFunction|SetBehavior "EAB_Nothing"))

(fn UpdateBehavior
  (if (and (Utilities|IsValid (Variables|Default|GetControlled%20MasterAI)) (Utilities|IsValid (Variables|Default|GetOwner%20Controller)))
    (if (Utilities|Enum|NotEqual(Enum) (Variables|/Script/TPMeleeCombat.StateManagerComponent|GetCurrentState (Variables|/Script/TPMeleeCombat.MasterAI|Getm_ACStateManagerComponent (Variables|Default|GetControlled%20MasterAI))) "ECS_Dead")
      (bind _output_get (LocalVariables|SetL_TargetActor (AI|BehaviorTree|GetBlackboardValueasActor (Variables|Default|GetTargetKey))))
      (Utilities|IsValid _output_get
        (:Is%20Valid
          (Variables|Default|SetbCanSeePlayer true)
          (LocalVariables|SetL_Distance (Transformation|GetDistanceTo (LocalVariables|GetL_TargetActor) (Variables|Default|GetControlled%20MasterAI)))
          (if (<= (LocalVariables|GetL_Distance) (Variables|Default|GetAttackingRange))
            (CallFunction|SetBehavior "EAB_Attacking")
            (else
              (CallFunction|SetBehavior "EAB_Chasing"))))
        (:Is%20Not%20Valid
          (CallFunction|SetBehavior "EAB_Patrolling")))
      (else
        (CallFunction|SetBehavior "EAB_Nothing")))))

(fn SetBehavior
  (params (NewBehavior :type EAIBehavior%20Enum :default "EAB_Nothing"))
  (Class|BTFunctionLibrary|SetBlackboardValueasEnum (Variables|Default|GetBehaviorKey) NewBehavior))