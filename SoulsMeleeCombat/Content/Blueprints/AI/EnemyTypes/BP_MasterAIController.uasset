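; BP_MasterAIController is the AI controller for BP_MasterAI pawns, relaying their combat state to the Blackboard.
; On possess, it casts and stores the pawn, then binds to the combat-enabled event of its MACCombatComponent.
; When that event fires, the handler writes the new state to the bCombatEnabled Blackboard key, so the controller needs no Tick logic.
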(event Custom|OnCombatToggled
  (params (bEnableCombat :type Boolean))
  (AI|Components|Blackboard|SetValueasBool (Variables|Default|GetBlackboard) (Utilities|Name|MakeLiteralName "bCombatEnabled") bEnableCombat))

(event EventBeginPlay)

(event EventTick
  (params (DeltaSeconds :type Float%20%28single-precision%29)))

(event EventPossess
  (params (PossessedPawn :type Pawn%20Object%20Reference))
  (bind _asbp_master_ai (Utilities|Casting|CastToBP_MasterAI PossessedPawn))
  (Variables|Default|SetAs%20BP%20Master%20AI _asbp_master_ai)
  (EventDispatchers|BindEventtoOnCombatEnabled (Variables|/Script/TPMeleeCombat.MasterAI|Getm_ACCombatComponent (Variables|Default|GetAs%20BP%20Master%20AI)) (delegate Custom|OnCombatToggled)))

(fn ConstructionScript)