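; Behavior tree task that makes a BP_MasterAI pawn perform an attack.
; It passes the attack type, index and random-index settings to PerformAttack on the pawn.
; It then waits for the returned duration plus an adjustable modifier before finishing successfully, with a leftover debug print at the start.
; A failed cast to BP_MasterAI never calls FinishExecute.
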(event EventReceiveExecuteAI
  (params (OwnerController :type AI%20Controller%20Object%20Reference) (ControlledPawn :type Pawn%20Object%20Reference))
  (Development|PrintString "Test" true true "(R=0.000000,G=0.660000,B=1.000000,A=1.000000)" 1.0)
  (bind _asbp_master_ai (Utilities|Casting|CastToBP_MasterAI ControlledPawn))
  (bind _output_get (Variables|Default|SetMasterAI _asbp_master_ai))
  (bind _returnvalue (Class|MasterAI|PerformAttack _output_get (Variables|Default|GetAttack%20Type) (Variables|Default|GetAttack%20Index) (Variables|Default|GetRandom%20Index)))
  (Utilities|FlowControl|Delay (+ _returnvalue (Variables|Default|GetAction%20Duration%20Modifier)))
  (AI|BehaviorTree|FinishExecute true))