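; Behavior tree task that makes a BP_MasterAI pawn perform an action, likely montage-driven, and holds the task until it ends.
; It passes montage index, random index, character action and state to the pawn's PerformAction.
; It delays by the returned value plus ActionDurationModifier, prints a debug string, then finishes successfully.
; A failed cast never calls FinishExecute, leaving the task running.
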(event EventReceiveExecuteAI
  (params (OwnerController :type AI%20Controller%20Object%20Reference) (ControlledPawn :type Pawn%20Object%20Reference))
  (bind _asbp_master_ai (Utilities|Casting|CastToBP_MasterAI ControlledPawn))
  (bind _output_get (Variables|Default|SetMasterAI _asbp_master_ai))
  (bind _returnvalue (Class|MasterAI|PerformAction _output_get (Variables|Default|GetMontage%20Index) (Variables|Default|GetRandom%20Index) (Variables|Default|GetChar%20Action) (Variables|Default|GetChar%20State)))
  (Utilities|FlowControl|Delay (+ _returnvalue (Variables|Default|GetAction%20Duration%20Modifier)))
  (Development|PrintString "Hello")
  (AI|BehaviorTree|FinishExecute true))