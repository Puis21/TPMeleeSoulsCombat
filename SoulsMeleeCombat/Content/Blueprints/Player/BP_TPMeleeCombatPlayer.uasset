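; Third-person melee combat player Blueprint that adds charge-attack input and debug tools.
; Left mouse press starts a looping timer that polls key hold time and fires ChargeAttackEvent once the charge threshold is reached.
; Tick optionally prints state, action and movement mode from the state manager and character, while Tab subtracts health through the stats component.
; PointDamage is an empty deprecated event, leaving its hit-reaction logic disconnected.
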(event Custom|TrackChargeAttBP
  (params (LMB :type Key%20Structure :default "None"))
  ;[0 1 0.2451] BP Charge Attack
  (Utilities|Time|SetTimerbyEvent (delegate Custom|ChargeAttackTimerEvent) 0.016 true))

(event Custom|ChargeAttackTimerEvent
  ;[0 1 0.2451] BP Charge Attack
  (bind _output_get (Variables|Default|Setm_fAttackHeldTime (Class|PlayerController|GetInputKeyTimeDown (Game|GetPlayerController 0) (stale Custom|TrackChargeAttBP LMB))))
  (bind _output_get_2 (Variables|Default|Setm_bIsAttackCharged (>= _output_get (Variables|Default|Getm_fChargeAttackTime))))
  (if _output_get_2
    (Utilities|Time|ClearTimerbyFunctionName 0 "ChargeAttackTimerEvent")
    (Class|TPMeleeCombatPlayer|ChargeAttackEvent)
    (Development|PrintString "Held" true false)))

(event EventBeginPlay)

(event Collision|EventActorBeginOverlap
  (params (OtherActor :type Actor%20Object%20Reference)))

(event EventTick
  (params (DeltaSeconds :type Float%20%28single-precision%29))
  (Utilities|FlowControl|Sequence
    (:then_0
      (if (Variables|Default|GetCanPrint)
        (Development|PrintString (Utilities|String|EnumtoString (Variables|/Script/TPMeleeCombat.StateManagerComponent|GetCurrentState (Variables|Default|Getm_ACStateManagerComponent))) true false "(R=0.000000,G=0.660000,B=1.000000,A=1.000000)" DeltaSeconds)))
    (:then_1
      (if (Variables|Default|GetCanPrint)
        (Development|PrintString (Utilities|String|EnumtoString (Variables|/Script/TPMeleeCombat.StateManagerComponent|GetCurrentAction (Variables|Default|Getm_ACStateManagerComponent))) true false "(R=1.000000,G=0.943894,B=0.000000,A=1.000000)" DeltaSeconds)))
    (:then_2
      (if (Variables|Default|GetCanPrint)
        (Development|PrintString (Utilities|String|EnumtoString (Variables|Default|GetMovementSpeedMode)) true false "(R=0.000000,G=1.000000,B=0.134428,A=1.000000)" DeltaSeconds)))))

(event EventTrackChargeAttack
  (params (Key :type Key%20Structure :default "None"))
  ;[0 1 0.2451] BP Charge Attack
)

(event Game|Damage|EventPointDamage
  (params (Damage :type Float%20%28single-precision%29) (DamageType :type Damage%20Type%20Object%20Reference) (HitLocation :type Vector :default "0, 0, 0") (HitNormal :type Vector :default "0, 0, 0") (HitComponent :type Primitive%20Component%20Object%20Reference) (BoneName :type Name :default "None") (ShotFromDirection :type Vector :default "0, 0, 0") (InstigatedBy :type Controller%20Object%20Reference) (DamageCauser :type Actor%20Object%20Reference) (HitInfo :type Hit%20Result%20Structure%20%28by%20ref%29))
  ;[0.9896 0.01734 0] DEPRECATED
)

(event EventClearChargeEventTimer
  ;[0 1 0.2451] BP Charge Attack
  (Utilities|Time|ClearTimerbyFunctionName 0 "ChargeAttackTimerEvent")
  (Development|PrintString "Timer" true false))

(event Input|MouseEvents|LeftMouseButton
  (params (Key :type Key%20Structure :default "None"))
  ;[0 1 0.2451] BP Charge Attack
  (:Pressed
    (CallFunction|TrackChargeAttBP Key)))

(event Input|KeyboardEvents|Tab
  (params (Key :type Key%20Structure :default "None"))
  (:Pressed
    (Class|StatsComponent|ModifyCurrentStatValue (Variables|Default|Getm_ACStatsComponent) "ES_Health" -25.0 true)))

(fn ConstructionScript)