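; BP_BaseDualWeapon is, by its name, a base Blueprint for dual-wielded player weapons, with main and left-hand collision components.
; Both components expose OnHit events, but neither runs any logic.
; Disconnected leftover nodes would print the hit actor's name or apply point damage from MFDamage along the owner's forward vector.
; BeginPlay, overlap, Tick and the construction script are also empty, so this graph adds no active behavior.
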(event OnHit(LeftHandCollisionComponent)
  (params (HitResult :type Hit%20Result%20Structure)))

(event OnHit(MainWeaponCollision)
  (params (HitResult :type Hit%20Result%20Structure)))

(event EventBeginPlay)

(event Collision|EventActorBeginOverlap
  (params (OtherActor :type Actor%20Object%20Reference)))

(event EventTick
  (params (DeltaSeconds :type Float%20%28single-precision%29)))

(fn ConstructionScript)